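; Game mode for local co-op play that gives each player a third-person character.
; On BeginPlay it creates local players up to NumberOfPlayers only when the game instance's PlayerStruct is empty.
; Each new player gets a character spawned at a player start and possessed, unless a populated PlayerStruct has no slot for its controller ID, in which case it is removed.
; A helper caches the GI_Cooperative reference.
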(event EventBeginPlay
  (if (Utilities|Array|IsEmpty (Variables|/Game/Cooperative/Core/GI_Cooperative.GI_Cooperative_C|GetPlayer%20Struct (CallFunction|GetGIRef)))
    (for _index (range 1 (Variables|Default|GetNumber%20Of%20Players))
      (Class|GameplayStatics|CreatePlayer _index))))

(event EventHandleStartingNewPlayer
  (params (NewPlayer :type Player%20Controller%20Object%20Reference))
  (bind _as_gi_coop (CallFunction|GetGIRef))
  (bind _player_struct (Variables|/Game/Cooperative/Core/GI_Cooperative.GI_Cooperative_C|GetPlayer%20Struct _as_gi_coop))
  (if (or (< (Class|GameplayStatics|GetPlayerControllerID NewPlayer) (Utilities|Array|Length _player_struct)) (Utilities|Array|IsEmpty _player_struct))
    (bind _returnvalue (Game|SpawnActorfromClass "/Game/Cooperative/Core/Game/BP_ThirdPersonCharacter.BP_ThirdPersonCharacter_C" (Math|Transform|MakeTransform (Transformation|GetActorLocation (Class|GameModeBase|FindPlayerStart NewPlayer)) "0, 0, 0" "1.000000,1.000000,1.000000") "Undefined" "MultiplyWithRoot" 0 0))
    (Pawn|Possess NewPlayer _returnvalue)
    (else
      (Class|GameplayStatics|RemovePlayer NewPlayer true))))

(fn ConstructionScript)

(fn GetGIRef
  ;[0.05098 0.05098 0.05098] Function for referencing the Game Instance
  (Variables|Default|GetAs%20GI%20Coop
    (:then
      _)
    (:else
      (bind _asgi_cooperative (Utilities|Casting|CastToGI_Cooperative (Game|GetGameInstance)))
      (Variables|Default|SetAs%20GI%20Coop _asgi_cooperative)))
  (return (Variables|Default|GetAs%20GI%20Coop)))