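; Main menu player controller for the cooperative lobby, where each player joins a slot, readies up or backs out, with sound feedback.
; Enhanced Input actions update slots through HUD_MainMenu and store ready players in GI_Cooperative, both reached through caching getters.
; The slot 0 player's ready triggers a one-second timer countdown shown on the menu widget, calling GS_MainMenu StartGame at zero.
; Backing out stops the countdown when the game instance's PlayerStruct is empty.
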(event Custom|Activar%20Temp
  ;[0.02083 0.02083 0.02083 0.036] Activación del temporizador
  (Default|ViewTemp (Variables|/Game/Cooperative/Core/MainMenu/HUD_MainMenu.HUD_MainMenu_C|GetW%20Main%20Menu (CallFunction|GetHudRef)))
  (Utilities|Time|SetTimerbyEvent (delegate Custom|Temp%20Funcionality) 1.0 (Variables|🕐Temporizador|GetTemporizador%20Activado)))

(event Custom|Temp%20Funcionality
  ;[0.02083 0.02083 0.02083 0.036] Funcionalidad del temporizador. Si los "Segundos" llegan a 0, se realizará un Cast al Game State del Main Menu y se ejecutará la función "Start Game"
  (if (== (Variables|🕐Temporizador|GetSegundos) 0)
    (bind _asgs_main_menu (Utilities|Casting|CastToGS_MainMenu (Game|GetGameState)))
    (Default|StartGame _asgs_main_menu)
    (else
      (if (Variables|🕐Temporizador|GetTemporizador%20Activado)
        (Variables|🕐Temporizador|SetSegundos (- (Variables|🕐Temporizador|GetSegundos) 1))
        (else
          (Utilities|FlowControl|DoOnce false
            (:Completed
              (Default|CloseTemp (Variables|/Game/Cooperative/Core/MainMenu/HUD_MainMenu.HUD_MainMenu_C|GetW%20Main%20Menu (CallFunction|GetHudRef)))
              (bind _output_get (Variables|🕐Temporizador|SetSegundos (Variables|🕐Temporizador|GetSegundosIniciales)))))))
      (Variables|/Game/Cooperative/UI/WBP_MainMenu.WBP_MainMenu_C|SetSegundos (Variables|/Game/Cooperative/Core/MainMenu/HUD_MainMenu.HUD_MainMenu_C|GetW%20Main%20Menu (CallFunction|GetHudRef)) _output_get))))

(event Custom|Restart%20Temp
  ;[0.02083 0.02083 0.02083 0.036] Funcionalidad del temporizador. Si los "Segundos" llegan a 0, se realizará un Cast al Game State del Main Menu y se ejecutará la función "Start Game"
  (Utilities|FlowControl|DoOnce false) ; enters at Reset
)

(event Input|EnhancedActionEvents|EnhancedInputActionIA_Action1
  (params (ActionValue :type Boolean) (ElapsedSeconds :type Float%20%28double-precision%29) (TriggeredSeconds :type Float%20%28double-precision%29) (InputAction :type Input%20Action%20Object%20Reference :default "/Game/Cooperative/Inputs/Actions/IA_Action1.IA_Action1"))
  (:Completed
    (Audio|PlaySound2D "/Game/Cooperative/Resources/Sounds/UserAccept.UserAccept" 1.0 1.0 0.0 0 0) ; Play Sound for "User Ready"
    ;[0.02083 0.02083 0.02083 0.036] Guardar el jugador en el mapa de "Players Ready" si le da a "Listo"
    (if (not (<= (Variables|Default|GetPlayer%20Slot) -1))
      (bind _playersready (Default|AddPlayerReady (CallFunction|GetHudRef)))
      (Variables|/Game/Cooperative/Core/GI_Cooperative.GI_Cooperative_C|SetPlayers%20Ready (CallFunction|GetGIRef) _playersready)
      ;[0.02083 0.02083 0.02083 0.036] Activar Temporizador
      (if (== (Variables|Default|GetPlayer%20Slot) 0)
        (Variables|🕐Temporizador|SetTemporizador%20Activado true)
        (CallFunction|ActivarTemp)))))

(event Input|EnhancedActionEvents|EnhancedInputActionIA_Action2
  (params (ActionValue :type Boolean) (ElapsedSeconds :type Float%20%28double-precision%29) (TriggeredSeconds :type Float%20%28double-precision%29) (InputAction :type Input%20Action%20Object%20Reference :default "/Game/Cooperative/Inputs/Actions/IA_Action2.IA_Action2"))
  (:Completed
    (Audio|PlaySound2D "/Game/Cooperative/Resources/Sounds/UserDisconnect.UserDisconnect" 1.0 1.0 0.0 0 0) ; Play Sound for "User Disconnect"
    (if (not (<= (Variables|Default|GetPlayer%20Slot) -1))
      ;[0.02083 0.02083 0.02083 0.036] Remove Slot
      (Default|RemovePlayerfromSlot (CallFunction|GetHudRef) (Variables|Default|GetPlayer%20Slot))
      ;[0.02083 0.02083 0.02083 0.036] Remove from Ready'sPlayer's
      (bind _player_slot_from_remove (Default|RemovePlayerfromReady'sPlayer (CallFunction|GetHudRef) (Variables|Default|GetPlayer%20Slot)))
      (Utilities|Map|Remove (Variables|/Game/Cooperative/Core/GI_Cooperative.GI_Cooperative_C|GetPlayers%20Ready (CallFunction|GetGIRef)) _player_slot_from_remove)
      ;[0.02083 0.02083 0.02083 0.036] Desactivar Temporizador
      (if (Utilities|Array|IsEmpty (Variables|/Game/Cooperative/Core/GI_Cooperative.GI_Cooperative_C|GetPlayer%20Struct (CallFunction|GetGIRef)))
        (Variables|🕐Temporizador|SetTemporizador%20Activado false)
        (CallFunction|RestartTemp)
        ;[0.02083 0.02083 0.02083 0.036] Eliminar slot del player
        (Variables|Default|SetPlayer%20Slot -1)))))

(event Input|EnhancedActionEvents|EnhancedInputActionIA_Start
  (params (ActionValue :type Boolean) (ElapsedSeconds :type Float%20%28double-precision%29) (TriggeredSeconds :type Float%20%28double-precision%29) (InputAction :type Input%20Action%20Object%20Reference :default "/Game/Cooperative/Inputs/Actions/IA_Start.IA_Start"))
  (:Completed
    (Audio|PlaySound2D "/Game/Cooperative/Resources/Sounds/UserConnect.UserConnect" 1.0 1.0 0.0 0 0) ; Play Sound for "User Connect"
    (if (<= (Variables|Default|GetPlayer%20Slot) -1)
      ;[0.02083 0.02083 0.02083 0.036] Añadir Player al slot correspondiente
      (bind _newplayerslot (Default|AddPlayertoSlot (CallFunction|GetHudRef)))
      (Variables|Default|SetPlayer%20Slot _newplayerslot))))

(event EventBeginPlay
  ;[0.02083 0.02083 0.02083 0.036 17] Establecer el "Enhanced Input Local Player Subsystem" con el nuevo sistema de inputs
  (Utilities|FlowControl|Delay 0.2)
  (Input|AddMappingContext (PlayerController|LocalPlayerSubsystems|GetEnhancedInputLocalPlayerSubsystem self) "/Game/Cooperative/Inputs/IMC_Default.IMC_Default" 0 "(bIgnoreAllPressedKeysUntilRelease=True,bForceImmediately=False)"))

(fn ConstructionScript)

(fn GetHudRef
  ;[0.02083 0.02083 0.02083 0.036] Function for referencing the HUD
  (Variables|Default|GetAs%20HUD%20Main%20Menu
    (:then
      _)
    (:else
      (bind _ashud_main_menu (Utilities|Casting|CastToHUD_MainMenu (HUD|GetHUD (Game|GetPlayerController 0))))
      (Variables|Default|SetAs%20HUD%20Main%20Menu _ashud_main_menu)))
  (return (Variables|Default|GetAs%20HUD%20Main%20Menu)))

(fn GetGIRef
  ;[0.02083 0.02083 0.02083 0.036] Function for referencing the Game Instance
  (Variables|Default|GetAs%20GI%20Coop
    (:then
      _)
    (:else
      (bind _asgi_cooperative (Utilities|Casting|CastToGI_Cooperative (Game|GetGameInstance)))
      (Variables|Default|SetAs%20GI%20Coop _asgi_cooperative)))
  (return (Variables|Default|GetAs%20GI%20Coop)))